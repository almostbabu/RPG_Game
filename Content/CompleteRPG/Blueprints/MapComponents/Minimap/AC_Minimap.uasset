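; AC_Minimap is an actor component that gives its owner a minimap by spawning and managing a BP_MinimapHandler actor.
; On BeginPlay a server event spawns the handler and passes it to the OC event, which stores it, sets its owner and attaches it to the component's owner.
; It also exposes validity-checked functions to set the minimap width and to read it from the handler's SceneCaptureComponent2D ortho width.
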(event Custom|SpawnActor%20-Server
  ;[1 1 1] Spawn Minimap Helper
  (bind _returnvalue (Game|SpawnActorfromClass "/Game/CompleteRPG/Blueprints/MapComponents/Minimap/BP_MinimapHandler.BP_MinimapHandler_C" (Math|Transform|MakeTransform "0, 0, 0" "0, 0, 0" "1,1,1") "Undefined" 0 0))
  (CallFunction|SpawnActor-OC _returnvalue))

(event Custom|SetCamWidth
  (params (OrthoWidth :type Float%20%28single-precision%29))
  (bind _spawnedactor (Variables|Default|GetSpawnedActor))
  ;[1 1 1] Set Minimap Width
  (Utilities|IsValid _spawnedactor
    (:Is%20Valid
      (Default|MinimapWidth _spawnedactor OrthoWidth))))

(event Custom|SpawnActor%20-OC
  (params (Target :type BP%20Minimap%20Handler%20Object%20Reference))
  (bind _returnvalue (Components|GetOwner))
  ;[1 1 1] Spawn Minimap Helper
  (Variables|Default|SetSpawnedActor Target)
  (Utilities|IsValid (Variables|Default|GetSpawnedActor)
    (:Is%20Valid
      (Utilities|IsValid (Variables|Default|GetSpawnedActor)
        (:Is%20Valid
          (Actor|SetOwner (Variables|Default|GetSpawnedActor) _returnvalue)
          (Transformation|AttachActorToActor (Variables|Default|GetSpawnedActor) _returnvalue "None" "KeepRelative" "KeepRelative" "KeepRelative" true))))))

(event EventBeginPlay
  ;[1 1 1] Start the Spawn
  (CallFunction|SpawnActor-Server))

(fn GetMinimapWidth
  (bind _spawnedactor (Variables|Default|GetSpawnedActor))
  (bind _scenecapturecomponent2d (Variables|/Game/CompleteRPG/Blueprints/MapComponents/Minimap/BP_MinimapHandler.BP_MinimapHandler_C|GetSceneCaptureComponent2D _spawnedactor))
  (Utilities|IsValid _spawnedactor
    (:Is%20Valid
      (Utilities|IsValid _scenecapturecomponent2d
        (:Is%20Valid
          (return (Variables|/Script/Engine.SceneCaptureComponent2D|GetOrthoWidth _scenecapturecomponent2d)))))))