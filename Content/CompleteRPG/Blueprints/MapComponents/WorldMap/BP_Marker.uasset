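; BP_Marker is a world map marker actor that shows its icon in the world through a widget component.
; On BeginPlay it initializes the WB_WorldActorWidget with itself, its marker texture and its owner.
; When a character with an AC_WorldMap component overlaps its sphere, it looks up its own index in that component and has the marker at that index removed.
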(event OnComponentBeginOverlap(Sphere)
  (params (OverlappedComponent :type Primitive%20Component%20Object%20Reference) (OtherActor :type Actor%20Object%20Reference) (OtherComp :type Primitive%20Component%20Object%20Reference) (OtherBodyIndex :type Integer) (bFromSweep :type Boolean) (SweepResult :type Hit%20Result%20Structure%20%28by%20ref%29))
  (bind _ascharacter (Utilities|Casting|CastToCharacter OtherActor))
  (Utilities|IsValid (Actor|GetComponentbyClass _ascharacter "/Game/CompleteRPG/Blueprints/MapComponents/WorldMap/AC_WorldMap.AC_WorldMap_C")
    (:Is%20Valid
      (bind _index (Default|GetMarkerIndexbyReference (Actor|GetComponentbyClass _ascharacter "/Game/CompleteRPG/Blueprints/MapComponents/WorldMap/AC_WorldMap.AC_WorldMap_C") self))
      (Default|RemoveMarkerIndex (Actor|GetComponentbyClass _ascharacter "/Game/CompleteRPG/Blueprints/MapComponents/WorldMap/AC_WorldMap.AC_WorldMap_C") _index))))

(event EventBeginPlay
  (bind _aswb_world_actor_widget (Utilities|Casting|CastToWB_WorldActorWidget (UserInterface|GetUserWidgetObject (Variables|Default|GetWidget))))
  (Default|Initialize _aswb_world_actor_widget self (Variables|Default|GetMarkerTexture) (Components|GetOwner)))

(fn ConstructionScript)