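; BP_InvItem is an interactable inventory item actor that destroys itself after being interacted with.
; Its construction script writes the Amount variable into the Item inventory struct.
; The ExecAfterInteract event gets the main widget handler component from the interacting object, hides the interact prompt widget, then calls DestroyEvent.
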(event EventBeginPlay
  (|CallParentFunction) ; This node is disabled and will not be called.\nDrag off pins to build functionality.
)

(event Collision|EventActorBeginOverlap
  (params (OtherActor :type Actor%20Object%20Reference)))

(event EventTick
  (params (DeltaSeconds :type Float%20%28single-precision%29)))

(event EventExecAfterInteract
  (Default|SetInteractWidgetVisibility (Actor|GetComponentbyClass (Variables|Default|GetInteractedVariable) "/Game/CompleteRPG/Blueprints/WidgetHandler/AC_MainWidgetHandler.AC_MainWidgetHandler_C") "Hidden" false "NewEnumerator0")
  (CallFunction|DestroyEvent))

(fn ConstructionScript
  (|CallParentFunction)
  (Utilities|Struct|SetmembersinS_ItemsInventory (Variables|Default|GetItem) (Variables|Default|GetAmount)))