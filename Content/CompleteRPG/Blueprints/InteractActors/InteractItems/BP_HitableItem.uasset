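; Hittable, targetable world item that rewards the attacker with an inventory item and reward alert on each hit.
; HandleHit plays effects and counts down hits until DestroyEvent hides the actor, makes it untargetable and toggles off the player's active target lock.
; If respawnable, a retriggerable delay restores it with full hits.
; The construction script takes its mesh from the rewarded item's info, and selection callbacks show or hide the target widget.
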(event Custom|DestroyEvent
  (Variables|Default|SetisDestroyed true)
  (Rendering|SetActorHiddenInGame true)
  (Variables|Default|SetTargetable? false)
  (CallFunction|TrytoRemoveTarget)
  (if (Variables|Default|GetRespawnable?)
    (Utilities|FlowControl|RetriggerableDelay (Variables|Default|GetRespawnTimer))
    (Variables|Default|SetCurrentHits (Variables|Hit|GetHits))
    (Rendering|SetActorHiddenInGame false)
    (Variables|Default|SetisDestroyed false)
    (Variables|Default|SetTargetable? true)))

(event EventBeginPlay
  (|CallParentFunction)
  (Variables|Default|SetCurrentHits (Variables|Hit|GetHits))
  (Utilities|FlowControl|Delay 1.5)
  (if (Variables|Default|GetisDestroyed)
    (Variables|Default|SetTargetable? false)))

(event Collision|EventActorBeginOverlap
  (params (OtherActor :type Actor%20Object%20Reference))
  (|CallParentFunction OtherActor) ; This node is disabled and will not be called.\nDrag off pins to build functionality.
)

(event EventTick
  (params (DeltaSeconds :type Float%20%28single-precision%29))
  (|CallParentFunction DeltaSeconds) ; This node is disabled and will not be called.\nDrag off pins to build functionality.
)

(fn ConstructionScript
  (bind _giveitemperhit (Variables|Hit|GetGiveItemPerHit))
  (bind _item (Utilities|Struct|BreakS_ItemsInventory _giveitemperhit))
  (bind _output_get (CallFunction|GetItemInfo _item))
  (bind _mesh (Utilities|Struct|BreakS_ItemStatic _output_get))
  (|CallParentFunction)
  (Utilities|IsValid _mesh
    (:Is%20Valid
      (Components|StaticMesh|SetStaticMesh (Variables|Default|GetStaticMesh) _mesh))))

(fn TrytoRemoveTarget
  (bind _player (Variables|Default|GetPlayer))
  (bind _returnvalue (Actor|GetComponentbyClass _player "/Game/CompleteRPG/Blueprints/Player/AC_FocusTarget.AC_FocusTarget_C"))
  (Utilities|IsValid _player
    (:Is%20Valid
      (Utilities|IsValid _returnvalue
        (:Is%20Valid
          (if (Default|IsTargetingEnabled _returnvalue)
            (Default|ToggleCameraLock _returnvalue)))))))

(fn TryEmitter
  (params (Location :type Vector))
  (bind _emitter (Variables|Default|GetEmitter))
  (Utilities|IsValid _emitter
    (:Is%20Valid
      (Effects|SpawnEmitteratLocation _emitter Location))))

(fn HandleHit
  (params (HitResult :type Hit%20Result%20Structure) (damage :type Float%20%28single-precision%29) (attack%20type :type E_AttackType%20Enum :default "NewEnumerator6") (weapon%20type :type E_WeaponType%20Enum :default "NewEnumerator5") (damage%20dealer :type Actor%20Object%20Reference) (WasCritical? :type Boolean) (Effects :type S%20Effect%20Chances%20Structure))
  (if (not (Variables|Default|GetisDestroyed))
    (Variables|Default|SetPlayer damage%20dealer)
    (CallFunction|TryEmitter (.Location (Collision|BreakHitResult HitResult)))
    (Audio|PlaySoundatLocation (Variables|Default|GetHitSound) (Transformation|GetActorLocation))
    (Utilities|IsValid (Variables|Default|GetPlayer)
      (:Is%20Valid
        (Utilities|IsValid (Actor|GetComponentbyClass (Variables|Default|GetPlayer) "/Game/CompleteRPG/Blueprints/MapComponents/PlayerState/AC_Inventory.AC_Inventory_C")
          (:Is%20Valid
            (Default|AddItem (Actor|GetComponentbyClass (Variables|Default|GetPlayer) "/Game/CompleteRPG/Blueprints/MapComponents/PlayerState/AC_Inventory.AC_Inventory_C") (Variables|Hit|GetGiveItemPerHit)))
          (:Is%20Not%20Valid
            _))
        (Utilities|IsValid (Actor|GetComponentbyClass (Variables|Default|GetPlayer) "/Game/CompleteRPG/Blueprints/WidgetHandler/AC_MainWidgetHandler.AC_MainWidgetHandler_C")
          (:Is%20Valid
            (Utilities|IsValid (Variables|/Game/CompleteRPG/Blueprints/WidgetHandler/AC_MainWidgetHandler.AC_MainWidgetHandler_C|GetRewardsAlert (Actor|GetComponentbyClass (Variables|Default|GetPlayer) "/Game/CompleteRPG/Blueprints/WidgetHandler/AC_MainWidgetHandler.AC_MainWidgetHandler_C"))
              (:Is%20Valid
                (Default|NewItemSlot (Variables|/Game/CompleteRPG/Blueprints/WidgetHandler/AC_MainWidgetHandler.AC_MainWidgetHandler_C|GetRewardsAlert (Actor|GetComponentbyClass (Variables|Default|GetPlayer) "/Game/CompleteRPG/Blueprints/WidgetHandler/AC_MainWidgetHandler.AC_MainWidgetHandler_C")) (Variables|Hit|GetGiveItemPerHit)))
              (:Is%20Not%20Valid
                _)))
          (:Is%20Not%20Valid
            _))
        (bind _result (Math|Integer|DecrementInt (Variables|Default|GetCurrentHits))
          (:%20%20
            (if (<= _result 0)
              (CallFunction|DestroyEvent)
              (return true)
              (else
                (return true)))))))))

(fn IsTargetable
  (return (Variables|Default|GetTargetable?)))

(fn OnDeselected
  (bind _targetwidget (Variables|Default|GetTargetWidget))
  (Utilities|IsValid _targetwidget
    (:Is%20Valid
      (Development|SetHiddeninGame _targetwidget true false)
      (return false))))

(fn OnSelected
  (bind _targetwidget (Variables|Default|GetTargetWidget))
  (Utilities|IsValid _targetwidget
    (:Is%20Valid
      (Development|SetHiddeninGame _targetwidget false false)
      (return false))))