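; BP_BagWithNeckle is a quest-gated interactable, apparently a bag tied to a necklace quest.
; It overrides Interact-ALL and acts only if the interacting player's AC_QuestsHandler finds the current quest from its ACQuestActor.
; It then runs the parent interaction and calls SetNewQuestInActor on that handler, targeting the Neckler reference at the first dialogue part with itself as the finished actor.
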(event EventBeginPlay
  (|CallParentFunction) ; This node is disabled and will not be called.\nDrag off pins to build functionality.
)

(event Collision|EventActorBeginOverlap
  (params (OtherActor :type Actor%20Object%20Reference))
  (|CallParentFunction OtherActor) ; This node is disabled and will not be called.\nDrag off pins to build functionality.
)

(event EventTick
  (params (DeltaSeconds :type Float%20%28single-precision%29))
  (|CallParentFunction DeltaSeconds) ; This node is disabled and will not be called.\nDrag off pins to build functionality.
)

(event EventInteract-ALL
  (params (InteractedVariable :type Character%20Object%20Reference))
  ;[1 1 1] Override Interact Event
  (Variables|Default|SetPlayer InteractedVariable)
  (bind _outputpin (Default|FindQuest (Actor|GetComponentbyClass (Variables|Default|GetPlayer) "/Game/CompleteRPG/Blueprints/MapComponents/AC_QuestsHandler.AC_QuestsHandler_C") (.Quest (Utilities|Struct|BreakS_QuestDynam (Variables|/Game/CompleteRPG/Blueprints/Quests/AC_QuestActor.AC_QuestActor_C|GetCurrentQuest (Variables|Default|GetAC_QuestActor))))))
  (if (!= _outputpin -1)
    (|CallParentFunction (Variables|Default|GetPlayer))
    (Default|SetNewQuestinActor (Actor|GetComponentbyClass (Variables|Default|GetPlayer) "/Game/CompleteRPG/Blueprints/MapComponents/AC_QuestsHandler.AC_QuestsHandler_C") (Variables|Default|GetNeckler) 0 self)))

(fn ConstructionScript
  (|CallParentFunction))