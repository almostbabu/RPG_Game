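; Actor component that detects melee weapon hits by tracing along mesh sockets while collision is active.
; Initialization takes all of the mesh's sockets or a supplied list and caches their world positions.
; Each tick it line-traces Pawns from each socket's previous position to its current one, then refreshes the cache.
; New hit actors fire OnHit once per activation, skipping the owner, already-hit actors and ignored classes.
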(event Custom|ActorsCollision
  (bind _actorshit (Variables|CollisionRegistration|GetActorsHit))
  ;[1 1 1] Reset Actors
  (Utilities|Array|Clear _actorshit)
  (Utilities|Array|Add _actorshit (Components|GetOwner))
  (Variables|CollisionRegistration|SetShouldPerformTrace? true))

(event Custom|DeactivateCollision
  ;[1 1 1] Collision Handle
  (Variables|CollisionRegistration|SetShouldPerformTrace? false))

(event Custom|SetSocketsLocation
  ;[1 1 1] Fill Sockets Previous Locations
  (for _array_element (Variables|CollisionRegistration|GetSockets)
    (Utilities|Map|Add (Variables|CollisionRegistration|GetLastSocketLocations) _array_element (Transformation|GetSocketLocation (Variables|CollisionRegistration|GetPlayerMesh) _array_element))))

(event Custom|InitializeSockets
  (params (WeaponMesh :type Skeletal%20Mesh%20Component%20Object%20Reference) (Sockets :type Array%20of%20Names))
  ;[1 1 1] ComponentWithSockets
  (Variables|CollisionRegistration|SetPlayerMesh WeaponMesh)
  (Variables|CollisionRegistration|SetSockets Sockets)
  (CallFunction|SetSocketsLocation))

(event Custom|Initialize
  (params (WeaponMesh :type Skeletal%20Mesh%20Component%20Object%20Reference))
  ;[1 1 1] Initialize Component
  (bind _output_get (Variables|CollisionRegistration|SetPlayerMesh WeaponMesh))
  (Variables|CollisionRegistration|SetSockets (Transformation|GetAllSocketNames _output_get))
  (CallFunction|SetSocketsLocation))

(event Custom|TryHit
  ;[1 1 1] Try to hit an object
  (for _array_element (Variables|CollisionRegistration|GetSockets)
    (bind _outhits (Class|KismetSystemLibrary|LineTraceMultiforObjects (.Value (CallFunction|GetLineTrace _array_element)) (.ReturnValue (CallFunction|GetLineTrace _array_element)) (Utilities|Array|MakeArray "ObjectTypeQuery3") false (Variables|CollisionRegistration|GetActorsHit) "None" true "(R=1.000000,G=0.000000,B=0.000000,A=1.000000)" "(R=0.000000,G=1.000000,B=0.000000,A=1.000000)" 3.0))
    (for _array_element_2 _outhits
      (if (not (CallFunction|CanbeHited? (.HitActor (Collision|BreakHitResult _array_element_2))))
        (Utilities|Array|Add (Variables|CollisionRegistration|GetActorsHit) (.HitActor (Collision|BreakHitResult _array_element_2)))
        (Default|CallOnHit _array_element_2)))))

(event EventTick
  (params (DeltaSeconds :type Float%20%28single-precision%29))
  ;[1 1 1] Try to hit on tick
  (Utilities|FlowControl|Sequence
    (:then_0
      (if (Variables|CollisionRegistration|GetShouldPerformTrace?)
        (CallFunction|TryHit)))
    (:then_1
      (CallFunction|SetSocketsLocation))))

(fn ValidCalss
  (params (TestClass :type Actor%20Class%20Reference))
  (for _array_element (Variables|CollisionRegistration|GetIgnoredClasses)
    (if (or (Utilities|ClassIsChildOf TestClass _array_element) (Utilities|Array|ContainsItem (Variables|CollisionRegistration|GetIgnoredClasses) TestClass))
      (return true)))
  (return false))

(fn GetLineTrace
  (params (InSocketName :type Name))
  (return (.Value (Utilities|Map|Find (Variables|CollisionRegistration|GetLastSocketLocations) InSocketName)) (Transformation|GetSocketLocation (Variables|CollisionRegistration|GetPlayerMesh) InSocketName)))

(fn CanbeHited?
  (params (ItemToFind :type Actor%20Object%20Reference%20%28by%20ref%29))
  (return (or (Utilities|Array|ContainsItem (Variables|CollisionRegistration|GetActorsHit) ItemToFind) (CallFunction|ValidCalss (Utilities|GetClass ItemToFind)))))