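; AI controller for warrior enemies that runs the combat behavior tree and manages player target acquisition and loss through AI perception.
; Sensing an attackable player-controlled pawn sets it as the controlled warrior's target.
; Tick retriggers a ten-second delay while the target's first stimulus stays sensed, so the target clears once that grace period lapses.
; SetTarget writes or clears the blackboard target, and getters expose blackboard key names.
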(event OnTargetPerceptionUpdated(AIPerception)
  (params (Actor :type Actor%20Object%20Reference) (Stimulus :type AI%20Stimulus%20Structure))
  (bind _aspawn (Utilities|Casting|CastToPawn Actor))
  ;[1 1 1] Try to find target
  (Utilities|IsValid Actor
    (:Is%20Valid
      (if (Math|Boolean|ANDBoolean (Utilities|DoesObjectImplementInterface Actor "/Game/CompleteRPG/Blueprints/Other/Interfaces/BP_I_CanBeAttacked.BP_I_CanBeAttacked_C") (Pawn|IsPlayerControlled _aspawn) (.bSuccessfullySensed (Utilities|Struct|BreakAIStimulus Stimulus)))
        (bind _asbp_warrior_ai (Utilities|Casting|CastToBP_Warrior_AI (Pawn|GetControlledPawn)))
        (bind _output_get (Variables|Default|SetCurrentPawn _aspawn))
        (Default|SetTarget _asbp_warrior_ai _output_get)))))

(event EventBeginPlay
  ;[1 1 1] Start Behaviour Tree
  (AI|RunBehaviorTree "/Game/CompleteRPG/Blueprints/Combat/AI/Controll/BT_CombatAI.BT_CombatAI"))

(event EventTick
  (params (DeltaSeconds :type Float%20%28single-precision%29))
  (Utilities|IsValid (Variables|Default|GetCurrentPawn)
    (:Is%20Valid
      (bind _info (Class|AIPerceptionComponent|GetActorsPerception (Variables|Default|GetAIPerception) (Variables|Default|GetCurrentPawn)))
      (if (.bSuccessfullySensed (Utilities|Struct|BreakAIStimulus (Utilities|Array|Get(acopy) (.LastSensedStimuli (Utilities|Struct|BreakActorPerceptionBlueprintInfo _info)))))
        (Utilities|FlowControl|RetriggerableDelay 1e+01)
        (bind _asbp_warrior_ai (Utilities|Casting|CastToBP_Warrior_AI (Pawn|GetControlledPawn)))
        (Default|RemoveTarget _asbp_warrior_ai (Variables|Default|GetCurrentPawn))
        (Variables|Default|SetCurrentPawn 0)))))

(fn ConstructionScript)

(fn SetTarget
  (params (NewTarget :type Actor%20Object%20Reference) (Remove? :type Boolean))
  (bind _blackboard (Variables|Default|GetBlackboard))
  (Utilities|IsValid _blackboard
    (:Is%20Valid
      (if Remove?
        (AI|Components|Blackboard|SetValueasObject (Variables|Default|GetBlackboard) (Key|MyTargetKey) 0)
        (else
          (AI|Components|Blackboard|SetValueasObject _blackboard (Key|MyTargetKey) NewTarget))))))

(fn MyTargetKey
  (return (Variables|BlackboardKeys|GetTargetKey)))

(fn MyPatrolKey
  (return (Variables|BlackboardKeys|GetPatrolKey)))

(fn MyStatusKey
  (return (Variables|BlackboardKeys|GetStatusKey)))

(fn MyPatrolBehKey
  (return (Variables|BlackboardKeys|GetPatrolBehKey)))

(fn MyMovementKey
  (return (Variables|BlackboardKeys|GetMovementKey)))

(fn MyCombatKey
  (return (Variables|BlackboardKeys|GetCombatKey)))

(fn MyAttackKey
  (return (Variables|BlackboardKeys|GetAttackKey)))

(fn MyHealthKey
  (return (Variables|BlackboardKeys|GetHealthKey)))

(fn MyTargetRangeKey
  (return (Variables|BlackboardKeys|GetTragetRangeKey)))