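; BP_QuestPlaceHelper is a world actor that carries a WB_QuestPoint widget to mark a quest location.
; BeginPlay passes the owner's AC_WorldMap component to the widget.
; SetNewLocation moves the actor, copies its position into the widget and hides it near the world origin, while two duplicate events toggle visibility.
; Character-distance culling with a Markered override exists but is disconnected, and Tick is empty.
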(event Custom|ToggleVisibility
  (params (bNewVisibility :type Boolean))
  ;[1 1 1] Toggle Vis
  (Rendering|SetVisibility (Variables|Default|GetWidget) bNewVisibility false))

(event Custom|ToggleVis
  (params (bNewVisibility :type Boolean))
  ;[1 1 1] Toggle Vis
  (Rendering|SetVisibility (Variables|Default|GetWidget) bNewVisibility false))

(event Custom|SetNewLocation
  (params (NewLocation :type Vector))
  ;[1 1 1] New Actor Location
  (Transformation|SetActorLocation NewLocation false false)
  (bind _output_get (Variables|/Game/CompleteRPG/UI/Widgets/WorldMap/Quest/WB_QuestPoint.WB_QuestPoint_C|SetLocation (CallFunction|GetQuestWidget) (Transformation|GetActorLocation)))
  (if (Math|Vector|Equal(Vector) _output_get "0, 0,0.000000" 1.0)
    (Rendering|SetVisibility (Variables|Default|GetWidget) false false)))

(event EventBeginPlay
  ;[1 1 1] Begin Play
  (Variables|/Game/CompleteRPG/UI/Widgets/WorldMap/Quest/WB_QuestPoint.WB_QuestPoint_C|SetMapRef (CallFunction|GetQuestWidget) (Actor|GetComponentbyClass (Components|GetOwner) "/Game/CompleteRPG/Blueprints/MapComponents/WorldMap/AC_WorldMap.AC_WorldMap_C")))

(event EventTick
  (params (DeltaSeconds :type Float%20%28single-precision%29))
  ;[1 1 1] Event Tick Hide And Show
)

(fn ConstructionScript)

(fn GetQuestWidget
  (bind _aswb_quest_point (Utilities|Casting|CastToWB_QuestPoint (UserInterface|GetUserWidgetObject (Variables|Default|GetWidget))))
  (return _aswb_quest_point))