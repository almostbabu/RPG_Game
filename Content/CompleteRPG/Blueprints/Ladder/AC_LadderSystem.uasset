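; Actor component that lets a Character use BP_LadderBase ladders: mounting, climbing up and down, and getting off at either end.
; Mounting switches to flying movement, blocks foot IK and lerps the character onto the ladder on Tick.
; Move input applies vertical movement and drives a state machine, using sphere traces and volume overlaps to detect the ends.
; State changes play montages, with delays timing the return to idle or walking.
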(event Custom|StartAnimation
  (params (TargetLocation :type Vector) (TargetRotation :type Rotator))
  ;[1 1 1] Ladder Animations
  (Variables|Default|SetTargetLocation TargetLocation)
  (Variables|Default|SetTargetRotation TargetRotation)
  (Variables|Default|SetStartLocation (Transformation|GetActorLocation (Variables|Default|GetOwner)))
  (Variables|Default|SetStartRotation (Transformation|GetActorRotation (Variables|Default|GetOwner)))
  (Variables|Default|SetAlpha 0.0)
  (Utilities|FlowControl|Gate true) ; enters at Open
)

(event Custom|EndAnimation
  ;[1 1 1] Ladder Animations
  (Utilities|FlowControl|Gate true) ; enters at Close
)

(event EventBeginPlay
  ;[1 1 1] Initialize
  (bind _ascharacter (Utilities|Casting|CastToCharacter (Components|GetOwner)))
  (Variables|Default|SetOwner _ascharacter))

(event EventTick
  (params (DeltaSeconds :type Float%20%28single-precision%29))
  ;[1 1 1] Ladder Animations
  (Utilities|FlowControl|Gate true
    (:Exit
      (Variables|Default|SetAlpha (+ (Variables|Default|GetAlpha) 0.05))
      (Transformation|SetActorLocationAndRotation (Variables|Default|GetOwner) (Math|Vector|Lerp(Vector) (Variables|Default|GetStartLocation) (Variables|Default|GetTargetLocation) (Variables|Default|GetAlpha)) (Math|Rotator|Lerp(Rotator) (Variables|Default|GetStartRotation) (Variables|Default|GetTargetRotation) (Variables|Default|GetAlpha) true))
      (if (>= (Variables|Default|GetAlpha) 1.0)
        (CallFunction|EndAnimation)))))

(fn Move
  (params (Value :type Float%20%28single-precision%29))
  (bind _owner (Variables|Default|GetOwner))
  (bind _returnvalue (Transformation|GetVelocity _owner))
  ;[1 1 1] Move On The Ladder
  (bind _output_get (LocalVariables|SetL_FA Value))
  (if (!= _output_get 0.0)
    (Variables|Booleans|SetInAir? (!= (.z _returnvalue) 0.0))
    (if (Variables|Booleans|GetInLadderArea)
      (if (Class|AnimInstance|IsAnyMontagePlaying (Components|SkeletalMesh|GetAnimInstance (Variables|/Script/Engine.Character|GetMesh (Variables|Default|GetOwner))))
        (return)
        (elif (Variables|Booleans|GetOnLadder)
          (CallFunction|ChangeCamRotation)
          (if (CallFunction|IsonTop?)
            (Usage|ChangeLadderState "NewEnumerator1")
            (else
              (Usage|ChangeLadderState "NewEnumerator3")))
          (if (== (LocalVariables|GetL_FA) 0.0)
            (if (!= (.z (Transformation|GetVelocity (Variables|Default|GetOwner))) 0.0)
              _
              (else
                (return)))
            (elif (Variables|Booleans|GetPermissed?)
              (if (CallFunction|NotChangingState?)
                _
                (else
                  (return)))
              (else
                (return))))
          (Pawn|Input|AddMovementInput (Variables|Default|GetOwner) (Transformation|GetActorUpVector (Variables|Default|GetOwner)) (LocalVariables|GetL_FA) false)
          (if (< (LocalVariables|GetL_FA) 0.0)
            (if (CallFunction|TraceDown)
              (Usage|ChangeLadderState "NewEnumerator8")
              (return)
              (else
                _))
            (elif (> (LocalVariables|GetL_FA) 0.0)
              (if (CallFunction|TraceUp)
                _
                (elif (CallFunction|InQuitArea?)
                  (Usage|ChangeLadderState "NewEnumerator2")
                  (return)
                  (else
                    (return))))))
          (if (> (LocalVariables|GetL_FA) 0.0)
            (Usage|ChangeLadderState "NewEnumerator6")
            (return)
            (elif (< (LocalVariables|GetL_FA) 0.0)
              (Usage|ChangeLadderState "NewEnumerator7")
              (return)
              (else
                (return))))
          (elif (Utilities|Enum|Equal(Enum) (Variables|State|GetCurrentState) "NewEnumerator0")
            _
            (else
              (Usage|ChangeLadderState "NewEnumerator0")
              (return))))))
    (return)
    (elif (== (.z _returnvalue) 0.0)
      (Usage|ChangeLadderState "NewEnumerator5"))))

(fn GetLocation
  (params (In :type Vector) (Socket :type Name))
  (bind (_x _y _z) (Math|Vector|BreakVector In))
  (bind _owner (Variables|Default|GetOwner))
  (bind _returnvalue (Transformation|GetActorLocation _owner))
  (bind _mesh (Variables|/Script/Engine.Character|GetMesh _owner))
  (bind _returnvalue_2 (Transformation|GetSocketLocation _mesh Socket))
  (return (Math|Vector|MakeVector (+ _x (.x _returnvalue)) (+ _y (.y _returnvalue)) (+ _z (.z _returnvalue))) (Math|Vector|MakeVector (+ _x (.x _returnvalue_2)) (+ _y (.y _returnvalue_2)) (+ _z (.z _returnvalue_2)))))

(fn CanLockinLadder
  (bind _owner (Variables|Default|GetOwner))
  (bind _returnvalue (Transformation|GetVelocity _owner))
  (bind (_x _y _z) (Math|Vector|BreakVector _returnvalue))
  (return (Math|Boolean|ANDBoolean (Math|Float|InRange(Float) _x (- _x 0.1) (+ _x 0.1)) (== _y 0.0) (== _z 0.0) (Variables|Booleans|GetInLadderArea))))

(fn PlayerMovetoCenter
  (params (Ladder :type BP%20Ladder%20Base%20Object%20Reference))
  (bind _owner (Variables|Default|GetOwner))
  (bind _charactermovement (Variables|/Script/Engine.Character|GetCharacterMovement _owner))
  (Variables|/Script/Engine.CharacterMovementComponent|SetBrakingDecelerationFlying (Variables|/Script/Engine.Character|GetCharacterMovement (Variables|Default|GetOwner)) 2048.0)
  (Variables|/Script/Engine.CharacterMovementComponent|SetMaxFlySpeed _charactermovement 2e+02)
  (Pawn|Components|CharacterMovement|SetMovementMode _charactermovement "MOVE_Flying" 0)
  (if (Variables|Booleans|GetInCenter)
    _
    (else
      (Components|Movement|StopMovementImmediately (Variables|/Script/Engine.Character|GetCharacterMovement (Variables|Default|GetOwner)))))
  (if (Utilities|Enum|NotEqual(Enum) (Variables|State|GetCurrentState) "NewEnumerator2")
    (CallFunction|StartAnimation (select (CallFunction|IsonTop?) (CallFunction|GetTopLocation Ladder) (CallFunction|GetBottomLocation Ladder)) (Transformation|GetWorldRotation (Variables|/Game/CompleteRPG/Blueprints/Ladder/BP_LadderBase.BP_LadderBase_C|GetVolume Ladder)))
    (Variables|Booleans|SetInCenter true)
    (Usage|ChangeLadderState "NewEnumerator1")))

(fn ChangeLadderState
  (params (Type :type Enum_LadderState%20Enum :default "NewEnumerator0"))
  (Variables|State|SetLocalState Type)
  (Utilities|FlowControl|Sequence
    (:then_0
      (if (and (Utilities|Enum|NotEqual(Enum) (Variables|State|GetCurrentState) (Variables|State|GetLocalState)) (or (Utilities|Enum|NotEqual(Enum) (Variables|State|GetCurrentState) "NewEnumerator2") (Utilities|Enum|NotEqual(Enum) (Variables|State|GetCurrentState) "NewEnumerator8")))
        (switch Utilities|FlowControl|Switch|SwitchonEnum_LadderState (Variables|State|GetLocalState)
          (:NewEnumerator0
            (Usage|Refresh))
          (:NewEnumerator1
            (if (or (Utilities|Enum|Equal(Enum) (Variables|State|GetCurrentState) "NewEnumerator6") (Utilities|Enum|Equal(Enum) (Variables|State|GetCurrentState) "NewEnumerator7")) :!label _label
              (Variables|State|SetLocalState "NewEnumerator5")
              (Variables|State|SetCurrentState (Variables|State|GetLocalState))
              (elif (Utilities|Enum|Equal(Enum) (Variables|State|GetCurrentState) "NewEnumerator0")
                (Variables|State|SetCurrentState (Variables|State|GetLocalState)))))
          (:NewEnumerator2
            (Variables|State|SetCurrentState (Variables|State|GetLocalState) :!label _label_2))
          (:NewEnumerator3
            (goto _label))
          (:NewEnumerator5
            (goto _label_2))
          (:NewEnumerator6
            (goto _label_2))
          (:NewEnumerator7
            (goto _label_2))
          (:NewEnumerator8
            (goto _label_2)))))
    (:then_1
      (CallFunction|OnStateChanged))))

(fn Refresh
  (Variables|Booleans|SetOnLadder false)
  (Variables|Booleans|SetPermissed? false)
  (Variables|Booleans|SetInCenter false)
  (Pawn|Components|CharacterMovement|SetMovementMode (Variables|/Script/Engine.Character|GetCharacterMovement (Variables|Default|GetOwner)) "MOVE_Walking" 0)
  (Variables|State|SetCurrentState "NewEnumerator0")
  (Variables|Booleans|SetCanMoveRight true)
  (Variables|/Script/Engine.CharacterMovementComponent|SetBrakingDecelerationFlying (Variables|/Script/Engine.Character|GetCharacterMovement (Variables|Default|GetOwner)) 0.0))

(fn StartClimbing
  (params (CurrentLadder :type BP%20Ladder%20Base%20Object%20Reference))
  (Variables|Booleans|SetInLadderArea true)
  (Variables|Default|SetCurrentLadder CurrentLadder)
  (Variables|Booleans|SetInCenter false))

(fn StopClimbing
  (Usage|Refresh)
  (Variables|Default|SetCurrentLadder 0)
  (Variables|Booleans|SetInLadderArea false))

(fn EnterLadderEnd
  (params (CurrentLadder :type BP%20Ladder%20Base%20Object%20Reference))
  (Variables|Default|SetCurrentLadder CurrentLadder))

(fn TrytoClimb
  (params (CurrentLadder :type BP%20Ladder%20Base%20Object%20Reference))
  (if (Variables|Booleans|GetOnLadder)
    (Usage|Refresh)
    (CallFunction|EndClimbing)
    (else
      (CallFunction|StartUsing CurrentLadder))))

(fn AndOwnerMontagePlaying?
  (return (Class|AnimInstance|IsAnyMontagePlaying (Components|SkeletalMesh|GetAnimInstance (Variables|/Script/Engine.Character|GetMesh (Variables|Default|GetOwner))))))

(fn ChangeCamRotation
  (bind _owner (Variables|Default|GetOwner))
  (bind _returnvalue (Transformation|GetActorTransform _owner))
  (bind _returnvalue_2 (Pawn|GetControlRotation _owner :!class /Script/Engine.Pawn))
  (Pawn|SetControlRotation (Pawn|GetController (Variables|Default|GetOwner)) (Math|Rotator|MakeRotator (.roll _returnvalue_2) (.pitch _returnvalue_2) (Math|Float|ClampAngle (.yaw _returnvalue_2) (- (.yaw (.rotation _returnvalue)) 9e+01) (+ (.yaw (.rotation _returnvalue)) 9e+01)))))

(fn TraceUp
  (bind _headsocket (Variables|Default|GetHeadSocket))
  (bind _withsocket (CallFunction|GetLocation "0, 0, 0" _headsocket))
  (bind (_x _y _z) (Math|Vector|BreakVector _withsocket))
  (bind _returnvalue (+ _z 1e+01))
  (bind _returnvalue_2 (Math|Vector|MakeVector _x _y _returnvalue))
  (bind (_outhit _returnvalue_3) (Collision|SphereTraceByChannel _returnvalue_2 (+ _returnvalue_2 (* (Transformation|GetActorForwardVector (Variables|Default|GetOwner)) 1.3e+02)) 5.0 "TraceTypeQuery1" false (Utilities|Array|MakeArray (Variables|Default|GetOwner)) "None"))
  (if _returnvalue_3
    (bind _asbp_ladder_base (Utilities|Casting|CastToBP_LadderBase (.HitActor (Collision|BreakHitResult _outhit)))
      (:then
        (return (Utilities|IsValid _asbp_ladder_base)))
      (:CastFailed
        (return false)))
    (else
      (return false))))

(fn TraceDown
  (bind _owner (Variables|Default|GetOwner))
  (bind _returnvalue (Transformation|GetActorLocation _owner))
  (bind (_x _y _z) (Math|Vector|BreakVector _returnvalue))
  (bind _returnvalue_2 (Collision|SphereTraceByChannel _returnvalue (Math|Vector|MakeVector _x _y (- _z 9e+01)) 5.0 "TraceTypeQuery1" false 0 "None"))
  (return _returnvalue_2))

(fn GetTopLocation
  (params (Target :type BP%20Ladder%20Base%20Object%20Reference))
  (bind _volume (Variables|/Game/CompleteRPG/Blueprints/Ladder/BP_LadderBase.BP_LadderBase_C|GetVolume Target))
  (bind _returnvalue (Transformation|GetWorldLocation _volume))
  (return (+ (Math|Vector|MakeVector (.x _returnvalue) (.y _returnvalue) (- (.z (Transformation|GetActorLocation (Variables|Default|GetOwner))) 165.0)) (* (Math|Vector|GetForwardVector (Variables|/Game/CompleteRPG/Blueprints/Ladder/BP_LadderBase.BP_LadderBase_C|GetVolume Target)) -5.0))))

(fn GetBottomLocation
  (params (Target :type BP%20Ladder%20Base%20Object%20Reference))
  (bind _volume (Variables|/Game/CompleteRPG/Blueprints/Ladder/BP_LadderBase.BP_LadderBase_C|GetVolume Target))
  (bind _returnvalue (Transformation|GetWorldLocation _volume))
  (return (Math|Vector|MakeVector (.x _returnvalue) (.y _returnvalue) (.z (Transformation|GetActorLocation (Variables|Default|GetOwner))))))

(fn EndClimbing
  (bind _owner (Variables|Default|GetOwner))
  (Variables|/Script/Engine.CharacterMovementComponent|SetbOrientRotationToMovement (Variables|/Script/Engine.Character|GetCharacterMovement (Variables|Default|GetOwner)) true)
  (Transformation|SetActorRotation _owner (Math|Rotator|MakeRotator 0.0 0.0 (.yaw (Transformation|GetActorRotation _owner))))
  (Variables|/Game/CompleteRPG/Blueprints/IK/AC_FootIK.AC_FootIK_C|SetForceBlocking (Actor|GetComponentbyClass (Components|GetOwner) "/Game/CompleteRPG/Blueprints/IK/AC_FootIK.AC_FootIK_C") false))

(fn StartUsing
  (params (CurrentLadder :type BP%20Ladder%20Base%20Object%20Reference))
  (if (not (Variables|Booleans|GetOnLadder))
    (bind _output_get (Variables|Default|SetCurrentLadder CurrentLadder))
    (CallFunction|PlayerMovetoCenter _output_get)
    (Variables|Booleans|SetOnLadder true)
    (Variables|Booleans|SetCanMoveRight false)
    (Variables|/Game/CompleteRPG/Blueprints/IK/AC_FootIK.AC_FootIK_C|SetForceBlocking (Actor|GetComponentbyClass (Components|GetOwner) "/Game/CompleteRPG/Blueprints/IK/AC_FootIK.AC_FootIK_C") true)))

(fn IsonTop?
  (return (Class|PrimitiveComponent|IsOverlappingComponent (Variables|/Script/Engine.Character|GetCapsuleComponent (Variables|Default|GetOwner)) (Variables|/Game/CompleteRPG/Blueprints/Ladder/BP_LadderBase.BP_LadderBase_C|GetTopVolume (Variables|Default|GetCurrentLadder)))))

(fn NotChangingState?
  (bind _currentstate (Variables|State|GetCurrentState))
  (return (or (Utilities|Enum|NotEqual(Enum) _currentstate "NewEnumerator3") (Utilities|Enum|NotEqual(Enum) _currentstate "NewEnumerator1"))))

(fn InQuitArea?
  (return (Class|PrimitiveComponent|IsOverlappingComponent (Variables|/Script/Engine.Character|GetCapsuleComponent (Variables|Default|GetOwner)) (Variables|/Game/CompleteRPG/Blueprints/Ladder/BP_LadderBase.BP_LadderBase_C|GetQuit (Variables|Default|GetCurrentLadder)))))

(fn GetQuitLocationandRotation
  (return (+ (Default|GetQuitLocation (Variables|Default|GetCurrentLadder)) (Math|Vector|MakeVector 0.0 0.0 (Components|Capsule|GetUnscaledCapsuleHalfHeight (Variables|/Script/Engine.Character|GetCapsuleComponent (Variables|Default|GetOwner))))) (Transformation|GetActorRotation (Variables|Default|GetOwner))))

(event Custom|OnStateChanged
  (bind (_location _rotation) (CallFunction|GetQuitLocationandRotation))
  ;[1 1 1] Play Event Montages
  (switch Utilities|FlowControl|Switch|SwitchonEnum_LadderState (Variables|State|GetCurrentState)
    (:NewEnumerator0
      (CallFunction|EndClimbing))
    (:NewEnumerator1
      (bind _returnvalue (Animation|PlayAnimMontage (Variables|Default|GetOwner) (Variables|Default|GetClimb_ON_Ladderr) 1.0 "" :!label _label))
      (Utilities|FlowControl|Delay (* _returnvalue (Variables|Default|GetAnimsDelayModifier)))
      (Variables|State|SetCurrentState "NewEnumerator5"))
    (:NewEnumerator2
      (bind _returnvalue_2 (Animation|PlayAnimMontage (Variables|Default|GetOwner) (Variables|Default|GetClimb_OFF_Ladder) 1.0 ""))
      (Variables|State|SetCurrentState "NewEnumerator0")
      (Utilities|FlowControl|Sequence
        (:then_0
          (Utilities|FlowControl|Delay _returnvalue_2)
          (Variables|Booleans|SetOnLadder false)
          (Usage|Refresh)
          (CallFunction|EndClimbing))
        (:then_1
          (Utilities|FlowControl|Delay (* _returnvalue_2 0.65))
          (CallFunction|StartAnimation _location _rotation))))
    (:NewEnumerator3
      (goto _label))
    (:NewEnumerator5
      (Variables|Booleans|SetPermissed? true))
    (:NewEnumerator6
      (Variables|/Script/Engine.CharacterMovementComponent|SetbOrientRotationToMovement (Variables|/Script/Engine.Character|GetCharacterMovement (Variables|Default|GetOwner)) false :!label _label_2))
    (:NewEnumerator7
      (goto _label_2))
    (:NewEnumerator8
      (Variables|Booleans|SetOnLadder false)
      (bind _returnvalue_3 (Animation|PlayAnimMontage (Variables|Default|GetOwner) (Variables|Default|GetClimb_FROM_Ladder) 1.0 ""))
      (Utilities|FlowControl|Delay (* _returnvalue_3 (Variables|Default|GetAnimsDelayModifier)))
      (Usage|Refresh)
      (CallFunction|EndClimbing))))