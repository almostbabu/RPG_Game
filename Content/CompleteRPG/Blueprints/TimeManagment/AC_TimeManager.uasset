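; Actor component on the player character that fast-forwards game time to a requested hour, apparently for meditation.
; SpeedupTime plays an optional sound, raises global time dilation, disables input and starts a looping timer that polls BP_WeatherManager's current hour.
; At the target hour it restores normal speed and input, clears the widget's Meditating flag, blends the view back and re-possesses the character.
; An unconnected debug branch spawns an overhead BP_TimeCamera.
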(event Custom|SpeedupTime
  (params (TimeToSpeedup :type Integer) (SpeedupWidget :type WB%20Speedup%20Time%20Object%20Reference))
  ;[1 1 1] Start Speedup Time Effect
  (Variables|Default|SetWidget SpeedupWidget)
  (Variables|Default|SetTimeToSpeedup TimeToSpeedup)
  (CallFunction|TryPlayTimeSound)
  (Utilities|Time|SetGlobalTimeDilation (Variables|Default|GetTimeDilation))
  (Input|DisableInput (Variables|Default|GetMainCharacter) (Variables|Default|GetPlayerController))
  (bind _returnvalue (Utilities|Time|SetTimerbyEvent (delegate Custom|EndTimeSpeedup) 0.01 true))
  (Variables|Default|SetTimer _returnvalue))

(event Custom|EndTimeSpeedup
  ;[1 1 1] Detect End Time Speedup Event
  (if (CallFunction|CanEndSpeedup)
    (Input|EnableInput (Variables|Default|GetMainCharacter) (Variables|Default|GetPlayerController))
    (Utilities|Time|PauseTimerbyHandle (Variables|Default|GetTimer))
    (Variables|/Game/CompleteRPG/UI/Widgets/Other/WB_SpeedupTime.WB_SpeedupTime_C|SetMeditating (Variables|Default|GetWidget) false)
    (Utilities|Time|SetGlobalTimeDilation 1.0)
    (Game|Player|SetViewTargetwithBlend (Variables|Default|GetPlayerController) (Variables|Default|GetMainCharacter) 1.0 "VTBlend_Linear" 0.0 false)
    (Utilities|FlowControl|Delay 0.8)
    (Pawn|Possess (Variables|Default|GetPlayerController) (Variables|Default|GetMainCharacter))))

(event EventBeginPlay
  ;[1 1 1] Initialize
  (bind _ascharacter (Utilities|Casting|CastToCharacter (Components|GetOwner)))
  (Variables|Default|SetMainCharacter _ascharacter)
  (bind _asplayer_controller (Utilities|Casting|CastToPlayerController (Pawn|GetController _ascharacter)))
  (Variables|Default|SetPlayerController _asplayer_controller))

(fn TryPlayTimeSound
  (bind _eventsound (Variables|Default|GetEventSound))
  (Utilities|IsValid _eventsound
    (:Is%20Valid
      (Audio|PlaySoundatLocation _eventsound (Transformation|GetActorLocation (Variables|Default|GetMainCharacter)) "0, 0, 0" 1.0 1.0 0.0 0 0 0))))

(fn CanEndSpeedup
  (bind _outactors (Actor|GetAllActorsOfClass "/Game/CompleteRPG/Blueprints/Weather/BP_WeatherManager.BP_WeatherManager_C"))
  (return (== (.Hours (Utilities|Struct|BreakS_FTime (Variables|/Game/CompleteRPG/Blueprints/Weather/BP_WeatherManager.BP_WeatherManager_C|GetMCurrentTime (Utilities|Array|Get(acopy) _outactors)))) (Variables|Default|GetTimeToSpeedup))))