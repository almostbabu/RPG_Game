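; Player controller for the CompleteRPG demo that lets the gamepad left stick move the mouse cursor.
; Stick directions act as digital press and release events that set the Right and Forward axis values.
; Tick adds those values to the current mouse position whenever either is non-zero, so the cursor steps one pixel per frame, independent of delta time.
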(event EventTick
  (params (DeltaSeconds :type Float%20%28single-precision%29))
  (bind (_locationx _locationy) (Game|Player|GetMousePosition))
  (|CallParentFunction DeltaSeconds)
  (if (or (!= (Variables|Default|GetRight) 0.0) (!= (Variables|Default|GetForward) 0.0))
    (Class|PlayerController|SetMouseLocation (Math|Float|Truncate (+ _locationx (Variables|Default|GetRight))) (Math|Float|Truncate (+ _locationy (Variables|Default|GetForward))))))

(event Input|GamepadEvents|GamepadLeftStickUp
  (params (Key :type Key%20Structure))
  (:Pressed
    (Variables|Default|SetForward -1.0))
  (:Released
    (Variables|Default|SetForward 0.0)))

(event Input|GamepadEvents|GamepadLeftStickDown
  (params (Key :type Key%20Structure))
  (:Pressed
    (Variables|Default|SetForward 1.0))
  (:Released
    (Variables|Default|SetForward 0.0)))

(event Input|GamepadEvents|GamepadLeftStickLeft
  (params (Key :type Key%20Structure))
  (:Pressed
    (Variables|Default|SetRight -1.0))
  (:Released
    (Variables|Default|SetRight 0.0)))

(event Input|GamepadEvents|GamepadLeftStickRight
  (params (Key :type Key%20Structure))
  (:Pressed
    (Variables|Default|SetRight 1.0))
  (:Released
    (Variables|Default|SetRight 0.0)))

(fn ConstructionScript)