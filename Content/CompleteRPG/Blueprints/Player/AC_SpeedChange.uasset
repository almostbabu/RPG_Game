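; Player component that controls movement speed for walk states such as walk, jog and run.
; ChangeWalkState reads a data table row, applies skill modifiers, then a looping timer eases speed, spring arm length and minimap width toward it.
; Tick scales that speed by SlowMod and a clamped inventory-weight and slope-angle factor, sending changes through a server event.
; StartInput also smooths movement input; GetCombatModifier is unused.
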(event Custom|StartInput
  (params (Target :type Pawn%20Object%20Reference) (WorldDirection :type Vector) (ScaleValue :type Float%20%28single-precision%29))
  ;[1 1 1] Smooth Walk
  (bind _output_get (Variables|Default|SetCurrentInput (Math|Interpolation|FInterpTo (Variables|Default|GetCurrentInput) ScaleValue (Utilities|Time|GetWorldDeltaSeconds) 1e+01)))
  (Pawn|Input|AddMovementInput Target WorldDirection _output_get false))

(event Custom|SetNewSpeed%20-Server
  (params (MaxWalkSpeed :type Float%20%28single-precision%29))
  ;[1 1 1] Change Speed
  (CallFunction|SetNewSpeed MaxWalkSpeed))

(event Custom|SetNewSpeed
  (params (MaxWalkSpeed :type Float%20%28single-precision%29))
  ;[1 1 1] Change Speed
  (Variables|/Script/Engine.CharacterMovementComponent|SetMaxWalkSpeed (Actor|GetComponentbyClass (Components|GetOwner) "/Script/Engine.CharacterMovementComponent") MaxWalkSpeed))

(event EventBeginPlay
  ;[1 1 1] Set start speed
  (Variables|Default|SetLastWalkSpeed (Variables|/Script/Engine.CharacterMovementComponent|GetMaxWalkSpeed (Actor|GetComponentbyClass (Components|GetOwner) "/Script/Engine.CharacterMovementComponent"))))

(event EventTick
  (params (DeltaSeconds :type Float%20%28single-precision%29))
  (bind _returnvalue (CallFunction|GetAngleSpeed))
  (bind _slowmod (Variables|Default|GetSlowMod))
  (bind _lastwalkspeed (Variables|Default|GetLastWalkSpeed))
  (bind _returnvalue_2 (* _lastwalkspeed _returnvalue _slowmod))
  (if (!= _returnvalue_2 (Variables|/Script/Engine.CharacterMovementComponent|GetMaxWalkSpeed (Actor|GetComponentbyClass (Components|GetOwner) "/Script/Engine.CharacterMovementComponent")))
    (CallFunction|SetNewSpeed-Server _returnvalue_2)))

(fn GetAngleSpeed
  (bind _returnvalue (Components|GetOwner))
  (bind _returnvalue_2 (Actor|GetComponentbyClass _returnvalue "/Game/CompleteRPG/Blueprints/AngleSpeed/AC_AngleSpeed.AC_AngleSpeed_C"))
  (bind _returnvalue_3 (Actor|GetComponentbyClass _returnvalue "/Game/CompleteRPG/Blueprints/MapComponents/PlayerState/AC_Inventory.AC_Inventory_C"))
  (bind _returnvalue_4 (Default|GetWeightAngle _returnvalue_3))
  (bind _newspeed (Default|AngleSpeedPerc _returnvalue_2))
  (bind _returnvalue_5 (+ _returnvalue_4 _newspeed))
  (Utilities|IsValid _returnvalue_3
    (:Is%20Valid
      (Utilities|IsValid _returnvalue_2
        (:Is%20Valid
          (return (Math|Float|Clamp(Float) (select (< _returnvalue_5 0.0) (+ (/ (Math|Float|Absolute(Float) _returnvalue_5) 1e+02) 1.0) (- 1.0 (/ _returnvalue_5 1e+02))) 0.15 3.0)))
        (:Is%20Not%20Valid
          _)))
    (:Is%20Not%20Valid
      _))
  (return 1.0))

(fn CanChangeSpeed
  (bind _returnvalue (Components|GetOwner))
  (bind _returnvalue_2 (Actor|GetComponentbyClass _returnvalue "/Game/CompleteRPG/Blueprints/Player/AC_PlayerCurrentState.AC_PlayerCurrentState_C"))
  (Utilities|IsValid _returnvalue
    (:Is%20Valid
      (Utilities|IsValid _returnvalue_2
        (:Is%20Valid
          (return (Utilities|Enum|NotEqual(Enum) (Variables|/Game/CompleteRPG/Blueprints/Player/AC_PlayerCurrentState.AC_PlayerCurrentState_C|GetCurrentState _returnvalue_2) "NewEnumerator1")))
        (:Is%20Not%20Valid
          _)))
    (:Is%20Not%20Valid
      _))
  (return true))

(fn ChangeWalkState
  (params (InputPin :type E_WalkState%20Enum :default "NewEnumerator3"))
  (bind (_newspeed _newspringarm _minimapwidth) (CallFunction|GetTypeSpeed InputPin))
  (if (CallFunction|CanChangeSpeed)
    (Variables|Default|SetTargetSpeed _newspeed)
    (Variables|Default|SetTargetSpringArm _newspringarm)
    (Variables|Default|SetTargetMinimap _minimapwidth)
    (bind _returnvalue (Utilities|Time|SetTimerbyFunctionName self "ChangeWalkTick" 0.016 true))
    (Variables|Default|SetSmoothlySpeedChangeHandle _returnvalue)))

(fn GetTypeSpeed
  (params (InputPin :type E_WalkState%20Enum :default "NewEnumerator3"))
  (bind _outrownames (DataTable|GetDataTableRowNames (Variables|Default|GetSpeed%20Data%20Table)))
  (for _array_element _outrownames
    (bind _returnvalue (Utilities|GetDataTableRow (Variables|Default|GetSpeed%20Data%20Table) _array_element)
      (:then
        (if (Utilities|Enum|Equal(Enum) (.Type (Utilities|Struct|BreakS_WalkState _returnvalue)) InputPin)
          (return (* (.Speed (Utilities|Struct|BreakS_WalkState _returnvalue)) (CallFunction|GetModifyer (.Type (Utilities|Struct|BreakS_WalkState _returnvalue)))) (.CamSpringArm (Utilities|Struct|BreakS_WalkState _returnvalue)) (.MinimapWidth (Utilities|Struct|BreakS_WalkState _returnvalue))))))))

(fn ChangeWalkTick
  (bind _returnvalue (Components|GetOwner))
  (bind _returnvalue_2 (Components|GetOwner))
  (bind _returnvalue_3 (Actor|GetComponentbyClass _returnvalue "/Game/CompleteRPG/Blueprints/MapComponents/Minimap/AC_Minimap.AC_Minimap_C"))
  (bind _returnvalue_4 (Actor|GetComponentbyClass _returnvalue_2 "/Script/Engine.SpringArmComponent"))
  (Utilities|IsValid _returnvalue_4
    (:Is%20Valid
      (Variables|/Script/Engine.SpringArmComponent|SetTargetArmLength _returnvalue_4 (Math|Interpolation|FInterpTo (Variables|/Script/Engine.SpringArmComponent|GetTargetArmLength _returnvalue_4) (Variables|Default|GetTargetSpringArm) (Utilities|Time|GetWorldDeltaSeconds) (Variables|Default|GetWalkInterpSpeed))))
    (:Is%20Not%20Valid
      _))
  (Utilities|IsValid _returnvalue_3
    (:Is%20Valid
      (Default|SetCamWidth _returnvalue_3 (Math|Interpolation|FInterpTo (Default|GetMinimapWidth _returnvalue_3) (Variables|Default|GetTargetMinimap) (Utilities|Time|GetWorldDeltaSeconds) (Variables|Default|GetWalkInterpSpeed))))
    (:Is%20Not%20Valid
      _))
  (bind _output_get (Variables|Default|SetLastWalkSpeed (Math|Interpolation|FInterpTo (Variables|Default|GetLastWalkSpeed) (Variables|Default|GetTargetSpeed) (Utilities|Time|GetWorldDeltaSeconds) (Variables|Default|GetWalkInterpSpeed))))
  (if (Math|Float|NearlyEqual(Float) _output_get (Variables|Default|GetTargetSpeed) 1.0)
    (Utilities|Time|ClearandInvalidateTimerbyHandle (Variables|Default|GetSmoothlySpeedChangeHandle))))

(fn GetModifyer
  (params (Type :type E_WalkState%20Enum :default "NewEnumerator3"))
  (bind _returnvalue (Components|GetOwner))
  (bind _runskill (Variables|Default|GetRunSkill))
  (bind _jogskill (Variables|Default|GetJogSkill))
  (bind _walkskill (Variables|Default|GetWalkSkill))
  (bind _returnvalue_2 (Actor|GetComponentbyClass _returnvalue "/Game/CompleteRPG/Blueprints/Skills/AC_Skills.AC_Skills_C"))
  (bind _returnvalue_3 (Utilities|Select :Index Type :NewEnumerator3 "" :NewEnumerator1 _runskill :NewEnumerator2 _jogskill :NewEnumerator0 _walkskill))
  (bind (_value _result) (Default|GetSkillValue _returnvalue_2 _returnvalue_3))
  (Utilities|IsValid _returnvalue_2
    (:Is%20Valid
      (if _result
        (return (+ (/ _value 1e+02) 1.0))
        (else
          _)))
    (:Is%20Not%20Valid
      _))
  (return 1.0))

(fn GetCombatModifier
  (bind _returnvalue (Components|GetOwner))
  (bind _returnvalue_2 (Actor|GetComponentbyClass _returnvalue "/Game/CompleteRPG/Blueprints/Combat/AC_CombatEvents.AC_CombatEvents_C"))
  (return (select (Variables|/Game/CompleteRPG/Blueprints/Combat/AC_CombatEvents.AC_CombatEvents_C|GetWeaponMode _returnvalue_2) (Utilities|Select :Index (Variables|/Game/CompleteRPG/Blueprints/Combat/AC_CombatEvents.AC_CombatEvents_C|GetCombatType _returnvalue_2) :NewEnumerator2 1.0 :NewEnumerator0 0.5 :NewEnumerator1 1.0) 1.0)))