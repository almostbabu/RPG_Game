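; BP_TravelPoint is a discoverable travel point with a teleportation widget that appears during eagle events.
; Sphere overlap makes the character the owner, then routes through server and OC events to clear any player marker.
; On first visit, it registers the waypoint with the character's AC_WorldMap and marks the area discovered.
; With a valid area DataTable row, it also shows a new-area popup, updates teleportation widgets and recreates the compass.
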(event OnComponentBeginOverlap(Sphere)
  (params (OverlappedComponent :type Primitive%20Component%20Object%20Reference) (OtherActor :type Actor%20Object%20Reference) (OtherComp :type Primitive%20Component%20Object%20Reference) (OtherBodyIndex :type Integer) (bFromSweep :type Boolean) (SweepResult :type Hit%20Result%20Structure%20%28by%20ref%29))
  ;[1 1 1] Start Overlap Event
  (bind _ascharacter (Utilities|Casting|CastToCharacter OtherActor))
  (Actor|SetOwner _ascharacter)
  (CallFunction|Overlap-Server OtherActor))

(event Custom|Overlap%20-OC
  (params (InputPin :type Actor%20Object%20Reference))
  (bind _areainfo (Variables|Default|GetAreaInfo))
  (bind _wb_teleportation (Variables|Default|GetWB_Teleportation))
  (bind _area (Utilities|Struct|BreakS_AreaStateStat _areainfo))
  (bind (_datatable _rowname) (Utilities|Struct|BreakDataTableRowHandle _area))
  ;[1 1 1] Overlap with multiplayer support
  (if (.Discovered? (Utilities|Struct|BreakS_AreaStateStat (Variables|Default|GetAreaInfo)))
    (CallFunction|RemoveMarker)
    (else
      (CallFunction|RemoveMarker)
      (bind _ascharacter (Utilities|Casting|CastToCharacter InputPin))
      (Utilities|IsValid (Actor|GetComponentbyClass _ascharacter "/Game/CompleteRPG/Blueprints/MapComponents/WorldMap/AC_WorldMap.AC_WorldMap_C")
        (:Is%20Valid
          (Default|DescoverWaypoint (Actor|GetComponentbyClass _ascharacter "/Game/CompleteRPG/Blueprints/MapComponents/WorldMap/AC_WorldMap.AC_WorldMap_C") self)
          (Utilities|Struct|SetmembersinS_AreaStateStat _areainfo true)
          (Utilities|IsValid _datatable
            (:Is%20Valid
              (bind _returnvalue (Utilities|GetDataTableRow _datatable _rowname)
                (:then
                  (bind _returnvalue_2 (UserInterface|CreateWidget "/Game/CompleteRPG/UI/Widgets/AnnounceScreen/WB_NewArea.WB_NewArea_C" 0 (.Name (Utilities|Struct|BreakS_AreaInfoStat _returnvalue)) (.DescoverPoints (Utilities|Struct|BreakS_AreaInfoStat _returnvalue))))
                  (UserInterface|Viewport|AddtoViewport _returnvalue_2 0)
                  (Utilities|IsValid _wb_teleportation
                    (:Is%20Valid
                      (Variables|/Game/CompleteRPG/UI/Widgets/WorldMap/WB_TeleportationPoint.WB_TeleportationPoint_C|SetDiscovered _wb_teleportation true))
                    (:Is%20Not%20Valid
                      _))
                  (bind _aswb_teleportation_point (Utilities|Casting|CastToWB_TeleportationPoint (UserInterface|GetUserWidgetObject (Variables|Default|GetAreaWidget))))
                  (Variables|/Game/CompleteRPG/UI/Widgets/WorldMap/WB_TeleportationPoint.WB_TeleportationPoint_C|SetDiscovered _aswb_teleportation_point true)
                  (Utilities|IsValid (CallFunction|GetChracterCompass _ascharacter)
                    (:Is%20Valid
                      (Default|Recreate (CallFunction|GetChracterCompass _ascharacter)))))))))))))

(event Custom|Overlap%20-Server
  (params (InputPin :type Actor%20Object%20Reference))
  ;[1 1 1] Overlap with multiplayer support
  (CallFunction|Overlap-OC InputPin))

(event Custom|EagleEvent
  (bind _aswb_teleportation_point (CallFunction|GetTeleportationPoint))
  ;[1 1 1] Eagle Events
  (Variables|Default|SetinEagleEvent true)
  (Variables|/Game/CompleteRPG/UI/Widgets/WorldMap/WB_TeleportationPoint.WB_TeleportationPoint_C|SetMapRef _aswb_teleportation_point (Variables|Default|GetMapComp))
  (Variables|/Game/CompleteRPG/UI/Widgets/WorldMap/WB_TeleportationPoint.WB_TeleportationPoint_C|SetLocation _aswb_teleportation_point (Transformation|GetActorLocation))
  (Rendering|SetVisibility (Variables|Default|GetAreaWidget) true false))

(event Custom|EagleReversedEvent
  ;[1 1 1] Eagle Events
  (Variables|Default|SetinEagleEvent false)
  (Rendering|SetVisibility (Variables|Default|GetAreaWidget) false false))

(event EventBeginPlay
  ;[1 1 1] Set Discovered by default
  (Rendering|SetVisibility (Variables|Default|GetAreaWidget) false false)
  (Variables|/Game/CompleteRPG/UI/Widgets/WorldMap/WB_TeleportationPoint.WB_TeleportationPoint_C|SetDiscovered (CallFunction|GetTeleportationPoint) (.Discovered? (Utilities|Struct|BreakS_AreaStateStat (Variables|Default|GetAreaInfo)))))

(fn ConstructionScript
  (|CallParentFunction)
  (Components|Sphere|SetSphereRadius (Variables|Default|GetSphere) (Variables|Default|GetSphereRadius) true))

(fn GetTeleportationPoint
  (bind _aswb_teleportation_point (Utilities|Casting|CastToWB_TeleportationPoint (UserInterface|GetUserWidgetObject (Variables|Default|GetAreaWidget))))
  (return _aswb_teleportation_point))

(fn RemoveMarker
  (bind _aswb_teleportation_point (CallFunction|GetTeleportationPoint))
  (Utilities|IsValid _aswb_teleportation_point
    (:Is%20Valid
      (if (Variables|/Game/CompleteRPG/UI/Widgets/WorldMap/WB_TeleportationPoint.WB_TeleportationPoint_C|GetPlayerMarked _aswb_teleportation_point)
        (Default|ToggleMarkerState (Variables|Default|GetWB_Teleportation))))))

(fn GetChracterCompass
  (params (Target :type Actor%20Object%20Reference))
  (bind _returnvalue (Actor|GetComponentbyClass Target "/Game/CompleteRPG/Blueprints/WidgetHandler/AC_MainWidgetHandler.AC_MainWidgetHandler_C"))
  (bind _wb_maingui (Variables|/Game/CompleteRPG/Blueprints/WidgetHandler/AC_MainWidgetHandler.AC_MainWidgetHandler_C|GetWB_MainGUI _returnvalue))
  (bind _wb_compass (Variables|/Game/CompleteRPG/UI/Widgets/Menu/WB_MainGUI.WB_MainGUI_C|GetWB_Compass _wb_maingui))
  (Utilities|IsValid Target
    (:Is%20Valid
      (Utilities|IsValid _returnvalue
        (:Is%20Valid
          (Utilities|IsValid _wb_maingui
            (:Is%20Valid
              (Utilities|IsValid _wb_compass
                (:Is%20Valid
                  (return _wb_compass))))))))))