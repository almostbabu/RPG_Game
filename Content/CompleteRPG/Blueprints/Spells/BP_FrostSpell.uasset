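; BP_FrostSpell is a sustained area frost spell that damages and freezes characters around it while draining its owner's energy.
; On spawn it sizes its sphere using the owner's radius skill, starts a looping timer and attaches a wind sound that fades out on destruction.
; Each tick of that timer charges energy, then applies frost and magical damage to non-owner characters in CharactersArray, with owner skills adjusting cost, duration and damage.
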(event Custom|DamageOverlaped
  (Default|RemoveEnergy (Actor|GetComponentbyClass (Components|GetOwner) "/Game/CompleteRPG/Blueprints/Player/AC_PlayerCharaacteristics.AC_PlayerCharaacteristics_C") (- (Variables|Default|GetCost) (.Value (Default|GetSkillValue (Actor|GetComponentbyClass (Components|GetOwner) "/Game/CompleteRPG/Blueprints/Skills/AC_Skills.AC_Skills_C") (Variables|Default|GetEnergySkill)))))
  (for _array_element (Variables|Default|GetCharactersArray)
    (if (!= _array_element (Components|GetOwner))
      (Utilities|IsValid _array_element
        (:Is%20Valid
          (Utilities|IsValid (Actor|GetComponentbyClass _array_element "/Game/CompleteRPG/Blueprints/Player/AC_PlayerCharaacteristics.AC_PlayerCharaacteristics_C")
            (:Is%20Valid
              (Default|TrytoFrost (Actor|GetComponentbyClass _array_element "/Game/CompleteRPG/Blueprints/Player/AC_PlayerCharaacteristics.AC_PlayerCharaacteristics_C") (+ (Variables|Default|GetFrostDelay) (.Value (Default|GetSkillValue (Actor|GetComponentbyClass (Components|GetOwner) "/Game/CompleteRPG/Blueprints/Skills/AC_Skills.AC_Skills_C") (Variables|Default|GetDelaySkill)))))
              (bind _ascharacter (Utilities|Casting|CastToCharacter (Components|GetOwner)))
              (Default|RemoveHealth (Actor|GetComponentbyClass _array_element "/Game/CompleteRPG/Blueprints/Player/AC_PlayerCharaacteristics.AC_PlayerCharaacteristics_C") (+ (Variables|Default|GetDamage) (.Value (Default|GetSkillValue (Actor|GetComponentbyClass (Components|GetOwner) "/Game/CompleteRPG/Blueprints/Skills/AC_Skills.AC_Skills_C") (Variables|Default|GetDamageSkill)))) true _ascharacter))))
        (:Is%20Not%20Valid
          (Utilities|Array|RemoveItem (Variables|Default|GetCharactersArray) _array_element))))))

(event Custom|OnDestroyed_Event_0
  (params (DestroyedActor :type Actor%20Object%20Reference))
  (Audio|Components|Audio|FadeOut (stale EventBeginPlay _returnvalue) 1.0 0.0 "Linear" :!class /Script/Engine.AudioComponent))

(event EventBeginPlay
  (|CallParentFunction)
  (Components|Sphere|SetSphereRadius (Variables|Default|GetSphere) (+ (Variables|Default|GetSphereRadius) (.Value (Default|GetSkillValue (Actor|GetComponentbyClass (Components|GetOwner) "/Game/CompleteRPG/Blueprints/Skills/AC_Skills.AC_Skills_C") (Variables|Default|GetRadiusSkill)))) true)
  (Utilities|Time|SetTimerbyEvent (delegate Custom|DamageOverlaped) 0.2 true)
  (bind _returnvalue (Audio|SpawnSoundAttached "/Game/CompleteRPG/Sounds/Whoosh/S_SpellWind.S_SpellWind" (Variables|Default|GetParticleSystem) "None" "0, 0, 0" "0, 0, 0" "KeepRelativeOffset" false 1.0 1.0 0.0 0 0 false))
  (EventDispatchers|AssignOnDestroyed (delegate Custom|OnDestroyed_Event_0)))

(event EventTick
  (params (DeltaSeconds :type Float%20%28single-precision%29))
  (|CallParentFunction DeltaSeconds))

(fn ConstructionScript
  (|CallParentFunction))