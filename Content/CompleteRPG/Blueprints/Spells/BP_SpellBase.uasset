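; BP_SpellBase is a base spell Blueprint that tracks which characters are inside its area of effect.
; Sphere begin and end overlaps cast the other actor to Character and pass it to StartSpellEvent and EndSpellEvent.
; These events add the character to, or remove it from, CharactersArray, with no spell effect applied here.
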(event OnComponentBeginOverlap(Sphere)
  (params (OverlappedComponent :type Primitive%20Component%20Object%20Reference) (OtherActor :type Actor%20Object%20Reference) (OtherComp :type Primitive%20Component%20Object%20Reference) (OtherBodyIndex :type Integer) (bFromSweep :type Boolean) (SweepResult :type Hit%20Result%20Structure%20%28by%20ref%29))
  (bind _ascharacter (Utilities|Casting|CastToCharacter OtherActor))
  (CallFunction|StartSpellEvent _ascharacter))

(event OnComponentEndOverlap(Sphere)
  (params (OverlappedComponent :type Primitive%20Component%20Object%20Reference) (OtherActor :type Actor%20Object%20Reference) (OtherComp :type Primitive%20Component%20Object%20Reference) (OtherBodyIndex :type Integer))
  (bind _ascharacter (Utilities|Casting|CastToCharacter OtherActor))
  (CallFunction|EndSpellEvent _ascharacter))

(event Custom|StartSpellEvent
  (params (Character :type Character%20Object%20Reference))
  (Utilities|Array|Add (Variables|Default|GetCharactersArray) Character))

(event Custom|EndSpellEvent
  (params (Character :type Character%20Object%20Reference))
  (if (Utilities|Array|ContainsItem (Variables|Default|GetCharactersArray) Character)
    (Utilities|Array|RemoveItem (Variables|Default|GetCharactersArray) Character)))

(fn ConstructionScript
  (|CallParentFunction))