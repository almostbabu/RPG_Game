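; BP_SlowDown is a placeable area that slows actors passing through it.
; When an actor carrying an AC_SpeedChange component overlaps its box, that component's SlowMod drops by the configured Percent.
; Leaving the box resets SlowMod to 1.0 rather than restoring any earlier value.
; The construction script applies the configurable Mesh to the static mesh component.
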(event OnComponentBeginOverlap(Box)
  (params (OverlappedComponent :type Primitive%20Component%20Object%20Reference) (OtherActor :type Actor%20Object%20Reference) (OtherComp :type Primitive%20Component%20Object%20Reference) (OtherBodyIndex :type Integer) (bFromSweep :type Boolean) (SweepResult :type Hit%20Result%20Structure%20%28by%20ref%29))
  (bind _returnvalue (Actor|GetComponentbyClass OtherActor "/Game/CompleteRPG/Blueprints/Player/AC_SpeedChange.AC_SpeedChange_C"))
  ;[1 1 1] Slow Down
  (Utilities|IsValid OtherActor
    (:Is%20Valid
      (Utilities|IsValid _returnvalue
        (:Is%20Valid
          (Variables|/Game/CompleteRPG/Blueprints/Player/AC_SpeedChange.AC_SpeedChange_C|SetSlowMod _returnvalue (- 1.0 (/ (Variables|Settings|GetPercent) 1e+02))))))))

(event OnComponentEndOverlap(Box)
  (params (OverlappedComponent :type Primitive%20Component%20Object%20Reference) (OtherActor :type Actor%20Object%20Reference) (OtherComp :type Primitive%20Component%20Object%20Reference) (OtherBodyIndex :type Integer))
  (bind _returnvalue (Actor|GetComponentbyClass OtherActor "/Game/CompleteRPG/Blueprints/Player/AC_SpeedChange.AC_SpeedChange_C"))
  ;[1 1 1] Slow Down
  (Utilities|IsValid OtherActor
    (:Is%20Valid
      (Utilities|IsValid _returnvalue
        (:Is%20Valid
          (Variables|/Game/CompleteRPG/Blueprints/Player/AC_SpeedChange.AC_SpeedChange_C|SetSlowMod _returnvalue 1.0))))))

(fn ConstructionScript
  (Components|StaticMesh|SetStaticMesh (Variables|Default|GetStaticMesh) (Variables|Settings|GetMesh)))