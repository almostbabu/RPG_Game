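; Actor component that runs one damaging status effect at a time on its owning character.
; StartEffect looks up damage, visual type and particles in data tables by effect type, starts a looping damage timer and attaches emitters to mesh sockets.
; EndEffect pauses the timer and deactivates emitters, then a delayed DestroyEffects handles their cleanup and clears the active flag.
; AddEffectPoints and DeactivateEffects are empty stubs.
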(fn AddEffectPoints
  (params (Value :type Float%20%28single-precision%29) (Effect :type E_Effects%20Enum :default "NewEnumerator1")))

(fn StartEffect
  (params (InputPin :type E_Effects%20Enum :default "NewEnumerator1"))
  (Variables|Default|SetLastEvent InputPin)
  (if (not (Variables|Default|GetActiveEffect?))
    ;[1 1 1] Start Effect Logic
    (Variables|Default|SetCurrentDamage (.Damage (Utilities|Struct|BreakS_EffectsInformation (CallFunction|GetEffectInformation (Variables|Default|GetLastEvent)))))
    (bind _returnvalue (Utilities|Time|SetTimerbyFunctionName 0 "DamageEffect" (.DamageRate (Utilities|Struct|BreakS_EffectsInformation (CallFunction|GetEffectInformation (Variables|Default|GetLastEvent)))) true))
    (Variables|Default|SetDamageTimer _returnvalue)
    (Variables|Default|SetLastEventVisual (CallFunction|TranslateEnum (Variables|Default|GetLastEvent)))
    (Variables|Default|SetActiveEffect? true)
    (LocalVariables|SetParticleInformation (CallFunction|GetEffectParticleInfo (Variables|Default|GetLastEvent)))
    (CallFunction|StartEffect (Variables|Default|GetLastEvent))
    (for _index (range 0 (- (Utilities|Array|Length (Utilities|Struct|BreakS_ParticleEffect (LocalVariables|GetParticleInformation))) 1))
      (bind _ascharacter (Utilities|Casting|CastToCharacter (Components|GetOwner)))
      (bind _returnvalue_2 (Effects|SpawnEmitterAttached (Utilities|Struct|BreakS_ParticleEffect (LocalVariables|GetParticleInformation)) (Variables|/Script/Engine.Character|GetMesh _ascharacter) (Utilities|Array|Get(acopy) (Utilities|Struct|BreakS_ParticleEffect (LocalVariables|GetParticleInformation)) _index) "0, 0, 0" "0, 0, 0" (Utilities|Struct|BreakS_ParticleEffect (LocalVariables|GetParticleInformation)) "KeepRelativeOffset" false))
      (Utilities|Array|Add (Variables|Default|GetEmitters) _returnvalue_2))
    (return true)
    (else
      (return false))))

(fn EndEffect
  (Utilities|Time|PauseTimerbyHandle (Variables|Default|GetDamageTimer))
  (Variables|Default|SetEmittersToDelete (Variables|Default|GetEmitters))
  (Utilities|Time|SetTimerbyFunctionName 0 "DestroyEffects" 0.5)
  (for _array_element (Variables|Default|GetEmitters)
    (Utilities|IsValid _array_element
      (:Is%20Valid
        (Components|Activation|Deactivate _array_element))))
  (Utilities|Array|Clear (Variables|Default|GetEmitters)))

(fn TranslateEnum
  (params (LastEvent :type E_Effects%20Enum :default "NewEnumerator1"))
  (bind _outrownames (DataTable|GetDataTableRowNames (Variables|Default|GetEffectsDT)))
  (for _array_element _outrownames
    (bind _returnvalue (Utilities|GetDataTableRow (Variables|Default|GetEffectsDT) _array_element)
      (:then
        (if (Utilities|Enum|Equal(Enum) (.MainEfects (Utilities|Struct|BreakS_EffectsMapping _returnvalue)) LastEvent)
          (return (.VisualEffects (Utilities|Struct|BreakS_EffectsMapping _returnvalue))))))))

(fn GetEffectInformation
  (params (InputPin :type E_Effects%20Enum :default "NewEnumerator1"))
  (bind _outrownames (DataTable|GetDataTableRowNames "/Game/CompleteRPG/Blueprints/Information/Effects/DT_EffectsInformation.DT_EffectsInformation"))
  (for _array_element _outrownames
    (bind _returnvalue (Utilities|GetDataTableRow "/Game/CompleteRPG/Blueprints/Information/Effects/DT_EffectsInformation.DT_EffectsInformation" _array_element)
      (:then
        (if (Utilities|Enum|Equal(Enum) (.Type (Utilities|Struct|BreakS_EffectsInformation _returnvalue)) InputPin)
          (return _returnvalue))))))

(fn GetEffectParticleInfo
  (params (InputPin :type E_Effects%20Enum :default "NewEnumerator1"))
  (bind _outrownames (DataTable|GetDataTableRowNames "/Game/CompleteRPG/Blueprints/Information/PlayerInfo/Particles/DT_ParticleEffect.DT_ParticleEffect"))
  (for _array_element _outrownames
    (bind _returnvalue (Utilities|GetDataTableRow "/Game/CompleteRPG/Blueprints/Information/PlayerInfo/Particles/DT_ParticleEffect.DT_ParticleEffect" _array_element)
      (:then
        (if (Utilities|Enum|Equal(Enum) (.Type (Utilities|Struct|BreakS_ParticleEffect _returnvalue)) InputPin)
          (return _returnvalue))))))

(fn DamageEffect
  (Game|Damage|ApplyDamage (Components|GetOwner) (Variables|Default|GetCurrentDamage) 0 0))

(fn DestroyEffects
  (bind _emitterstodelete (Variables|Default|GetEmittersToDelete))
  (for _array_element _emitterstodelete
    (Utilities|IsValid _array_element
      (:Is%20Valid
        (Components|DestroyComponent _emitterstodelete))))
  (Variables|Default|SetActiveEffect? false)
  (Utilities|Array|Clear (Variables|Default|GetEmittersToDelete)))

(fn DeactivateEffects)