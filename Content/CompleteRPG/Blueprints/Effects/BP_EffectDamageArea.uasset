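; BP_EffectDamageArea is a trigger area that applies a configurable Effect to characters that enter its Box.
; On overlap begin it calls StartEffect on the character's AC_EffectHandle component, if present.
; On overlap end it stores LastCharacter and calls EndEffect after a retriggerable EffectEndDelay.
; Only the last character to leave within that delay gets EndEffect, and re-entering does not cancel it.
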(event OnComponentBeginOverlap(Box)
  (params (OverlappedComponent :type Primitive%20Component%20Object%20Reference) (OtherActor :type Actor%20Object%20Reference) (OtherComp :type Primitive%20Component%20Object%20Reference) (OtherBodyIndex :type Integer) (bFromSweep :type Boolean) (SweepResult :type Hit%20Result%20Structure%20%28by%20ref%29))
  ;[1 1 1] Toggle Effect
  (bind _ascharacter (Utilities|Casting|CastToCharacter OtherActor))
  (Utilities|IsValid (Actor|GetComponentbyClass _ascharacter "/Game/CompleteRPG/Blueprints/Effects/AC_EffectHandle.AC_EffectHandle_C")
    (:Is%20Valid
      (Default|StartEffect (Actor|GetComponentbyClass _ascharacter "/Game/CompleteRPG/Blueprints/Effects/AC_EffectHandle.AC_EffectHandle_C") (Variables|Default|GetEffect)))))

(event OnComponentEndOverlap(Box)
  (params (OverlappedComponent :type Primitive%20Component%20Object%20Reference) (OtherActor :type Actor%20Object%20Reference) (OtherComp :type Primitive%20Component%20Object%20Reference) (OtherBodyIndex :type Integer))
  ;[1 1 1] Toggle Effect
  (bind _ascharacter (Utilities|Casting|CastToCharacter OtherActor))
  (Variables|Default|SetLastCharacter _ascharacter)
  (Utilities|FlowControl|RetriggerableDelay (Variables|Default|GetEffectEndDelay))
  (Utilities|IsValid (Variables|Default|GetLastCharacter)
    (:Is%20Valid
      (Utilities|IsValid (Actor|GetComponentbyClass (Variables|Default|GetLastCharacter) "/Game/CompleteRPG/Blueprints/Effects/AC_EffectHandle.AC_EffectHandle_C")
        (:Is%20Valid
          (Default|EndEffect (Actor|GetComponentbyClass (Variables|Default|GetLastCharacter) "/Game/CompleteRPG/Blueprints/Effects/AC_EffectHandle.AC_EffectHandle_C")))))))

(fn ConstructionScript)